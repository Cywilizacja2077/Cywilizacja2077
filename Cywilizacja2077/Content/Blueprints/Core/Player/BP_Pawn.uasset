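; BP_Pawn is a player pawn that acts as a movable camera rig with spring-arm zoom.
; Forward and right axis inputs shift a desired location along the actor's facing, while the zoom axis adjusts a clamped desired arm length.
; Tick smoothly interpolates the actor location and spring arm length toward those targets, moving without sweep collision.
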(event `self.ReceiveBeginPlay`
  (set `self.Location_Desired` (`self.K2_GetActorLocation`))
  (set `self.Zoom_Desired` (`SpringArmComponent.TargetArmLength` (`self.SpringArm`))))

(event `InputAxis|InputAxis_Forward`
  (params (AxisValue :type "Float (single-precision)"))
  (set `self.Location_Desired` (+ (`self.Location_Desired`) (* (`self.GetActorForwardVector`) (* AxisValue (`self.Location_Speed`))))))

(event `InputAxis|InputAxir_Right`
  (params (AxisValue :type "Float (single-precision)"))
  (set `self.Location_Desired` (+ (`self.Location_Desired`) (* (`self.GetActorRightVector`) (* AxisValue (`self.Location_Speed`))))))

(event `InputAxis|InputAxis_Zoom`
  (params (AxisValue :type "Float (single-precision)"))
  (set `self.Zoom_Desired` (`KismetMathLibrary.FClamp` (+ (`self.Zoom_Desired`) (* AxisValue (`self.Zoom_Speed`))) (`self.Zoom_Min`) (`self.Zoom_Max`))))

(event `self.ReceiveTick`
  (params (DeltaSeconds :type "Float (single-precision)"))
  (bind _springarm (`self.SpringArm`))
  (set `SpringArmComponent.TargetArmLength` (`KismetMathLibrary.FInterpTo` (`SpringArmComponent.TargetArmLength` _springarm) (`self.Zoom_Desired`) DeltaSeconds (`self.Zoom_Interp`)) _springarm)
  (`self.K2_SetActorLocation` (`KismetMathLibrary.VInterpTo` (`self.K2_GetActorLocation`) (`self.Location_Desired`) DeltaSeconds (`self.Location_Interp`))))

(fn `UserConstructionScript`)