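; Grid actor that builds a flat hexagon tile grid as instanced static meshes in its construction script.
; SpawnGrid clears old instances, snaps the center to tile size, derives the bottom-left corner, then places tiles using doubled-row coordinates, offsetting alternate columns.
; Tile scale uses mesh size from a shape data table, though mesh and material are hardcoded to hexagon.
; Index-to-location mapping is marked temporary and includes a fixed X offset.
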(event `self.ReceiveBeginPlay`)

(event `self.ReceiveTick`
  (params (DeltaSeconds :type "Float (single-precision)")))

(fn `CalculateCenterAndBottomLeft`
  (returns (Center :type "Vector Structure") (BottomLeft :type "Vector Structure"))
  (locals (C :type "Vector Structure" :default (0.0 0.0 0.0)))
  (bind (_tile_count_x _tile_count_y) (`KismetMathLibrary.BreakVector2D` (`self.Tile Count`)))
  (set `local.C` (`/Game/Blueprints/Core/Utilities/BFL_Utilities.SnapVectorToVector` (`self.Center Location`) (* (`self.Tile Size`) (1.5 1.0 0.0))))
  (return (`local.C`) (- (`local.C`) (* (/ (- (`self.Tile Count`) (`KismetMathLibrary.MakeVector2D` (`KismetMathLibrary.SelectFloat` 0.0 1.0 (`/Game/Blueprints/Core/Utilities/BFL_Utilities.IsFloatEven` _tile_count_x)) (`KismetMathLibrary.SelectFloat` 0.0 1.0 (`/Game/Blueprints/Core/Utilities/BFL_Utilities.IsFloatEven` _tile_count_y)))) 2.0) (`KismetMathLibrary.Conv_VectorToVector2D` (`self.Tile Size`))))))

(fn `DestroyGrid`
  (params (self2 :type "InstancedStaticMeshComponent Object Reference"))
  (`InstancedStaticMeshComponent.ClearInstances` self2))

(fn `GetCurrentShapeData`
  (returns (ReturnValue :type "/Game/Blueprints/Core/Grid/GridShapes/S_GridShapeData Structure"))
  (bind _returnvalue (`|GetDataTableRow` "/Game/Blueprints/Core/Grid/GridShapes/DT_GridShapeData.DT_GridShapeData" (`KismetStringLibrary.Conv_StringToName` (`KismetStringLibrary.Conv_NameToString` (`|GetEnumeratorName` (`self.Shape`)))))
    (:`then`
      _)
    (:`RowNotFound`
      _))
  (return _returnvalue))

(fn `GetTileLocationFromIndex`
  (params (Index :type "Vector2D Structure"))
  (returns (ReturnValue :type "Vector Structure"))
  (return (+ (+ (`self.BottomLeftCornerLocation`) (* (`self.Tile Size`) (* Index (0.75 0.5)))) (200.0 0.0 0.0))))

(fn `SpawnGrid`
  (params (CenterLocation :type "Vector Structure") (TileSize :type "Vector Structure") (TileCount :type "Vector2D Structure") (Shape :type "/Game/Blueprints/Core/Grid/GridShapes/E_GridShape Enum" :default "NewEnumerator1"))
  (locals (X :type Integer) (Y :type Integer) (TileTransform :type "Transform Structure") (Index :type "Vector2D Structure"))
  (bind _instancedstaticmesh (`self.InstancedStaticMesh`))
  (bind (_tilecount_x _tilecount_y) (`KismetMathLibrary.BreakVector2D` (`local.TileCount`)))
  (bind (_tile_count_x _tile_count_y) (`KismetMathLibrary.BreakVector2D` (`self.Tile Count`)))
  (bind _tile_count_x_2 (`KismetMathLibrary.BreakVector2D` (`self.Tile Count`)))
  (set `self.Center Location` CenterLocation)
  (set `self.Tile Size` TileSize)
  (set `self.Shape` Shape)
  (set `self.Tile Count` (`KismetMathLibrary.MakeVector2D` (`KismetMathLibrary.Conv_IntToDouble` (`KismetMathLibrary.Round` _tilecount_x)) (`KismetMathLibrary.Conv_IntToDouble` (`KismetMathLibrary.Round` _tilecount_y))))
  (`self.DestroyGrid` (`self.InstancedStaticMesh`))
  (`StaticMeshComponent.SetStaticMesh` _instancedstaticmesh "/Game/Blueprints/Core/Grid/Hexagon/SM_Grid_HexagonFlat.SM_Grid_HexagonFlat")
  (`PrimitiveComponent.SetMaterial` _instancedstaticmesh 0 "/Game/Blueprints/Core/Grid/Hexagon/MI_Grid_Flat_Border_Hexagon.MI_Grid_Flat_Border_Hexagon")
  (bind (_center _bottomleft) (`self.CalculateCenterAndBottomLeft`))
  (set `self.Center Location` _center)
  (set `self.BottomLeftCornerLocation` _bottomleft)
  (for _index (range (`KismetMathLibrary.Round` _tile_count_x_2))
    (set `local.X` _index)
    (for _index_2 (range (`KismetMathLibrary.SelectInt` 0 1 (`/Game/Blueprints/Core/Utilities/BFL_Utilities.IsIntEven` (`local.X`))) (* (`KismetMathLibrary.Round` _tile_count_y) 2))
      (set `local.Y` _index_2)
      (`|ExecutionSequence`
        (:`then_0`
          (set `local.Index` (`KismetMathLibrary.MakeVector2D` (`KismetMathLibrary.Conv_IntToDouble` (`local.X`)) (`KismetMathLibrary.Conv_IntToDouble` (`local.Y`))))
          (set `local.TileTransform` (`KismetMathLibrary.MakeTransform` (`self.GetTileLocationFromIndex` (`local.Index`)) (struct) (/ (`self.Tile Size`) (`.MeshSize_2_03CF4F614C6324128B3DAE8CA0698EB8` (break `/Game/Blueprints/Core/Grid/GridShapes/S_GridShapeData` (`self.GetCurrentShapeData`))))))
          (`InstancedStaticMeshComponent.AddInstance` (`self.InstancedStaticMesh`) (`local.TileTransform`) true))
        (:`then_1`
          (`/Engine/EditorBlueprintResources/StandardMacros.IncrementInt` _index_2))))))

(fn `UserConstructionScript`
  (`self.SpawnGrid` (`self.K2_GetActorLocation`) (`self.Tile Size`) (`self.Tile Count`) (`self.Shape`)))