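; BP_Resources tracks each player's gold, wood, stone and food and shows the current player's totals on the HUD.
; Starting amounts come from DT_TeamResources rows and are appended to one flat TeamResources array of player, resource and amount entries.
; Reads assume each player's four entries are consecutive in that order, while ModifyResource adds to the entry matching player and type.
; CreateResourceMenu spawns the NewHUD actor and pushes the totals to its UI.
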(fn `Change Resource Menu Values`
  (bind (_gold _wood _stone _food) (`self.Get Team Resources`))
  (`/Game/Blueprints/Core/Resources/Widgets/MainHUD.Event Update Text` (`/Game/Blueprints/NewHUD.UI_Ref` (`self.Resource Ref`)) _gold _wood _stone _food))

(fn `Create Resource Menu`
  (bind _returnvalue (`|SpawnActorFromClass` "/Game/Blueprints/NewHUD.NewHUD_C" (`KismetMathLibrary.MakeTransform` (0.0 0.0 0.0)) "Undefined" "MultiplyWithRoot" null null))
  (set `self.Resource Ref` _returnvalue)
  (`self.Change Resource Menu Values`))

(fn `Get Team Resources`
  (returns (Gold :type Integer) (Wood :type Integer) (Stone :type Integer) (Food :type Integer))
  (locals (G :type Integer) (W :type Integer) (S :type Integer) (F :type Integer))
  (bind _team_resources (`self.Team Resources`))
  (for _index (range (`KismetArrayLibrary.Array_Length` (`self.Team Resources`)))
    (bind _output_player (break `/Game/Blueprints/Core/Resources/Utilities/S_TeamResources` (`|GetArrayItem` (`self.Team Resources`) _index)))
    (if (== (`self.CurrentPlayer`) _output_player)
      (bind (_output_player_2 _output_resource _output_amount) (break `/Game/Blueprints/Core/Resources/Utilities/S_TeamResources` (`|GetArrayItem` _team_resources _index)))
      (bind _output_get (set `local.G` _output_amount))
      (bind (_output_player_3 _output_resource_2 _output_amount_2) (break `/Game/Blueprints/Core/Resources/Utilities/S_TeamResources` (`|GetArrayItem` _team_resources (+ _index 1))))
      (bind _output_get_2 (set `local.W` _output_amount_2))
      (bind (_output_player_4 _output_resource_3 _output_amount_3) (break `/Game/Blueprints/Core/Resources/Utilities/S_TeamResources` (`|GetArrayItem` _team_resources (+ _index 2))))
      (bind _output_get_3 (set `local.S` _output_amount_3))
      (bind (_output_player_5 _output_resource_4 _output_amount_4) (break `/Game/Blueprints/Core/Resources/Utilities/S_TeamResources` (`|GetArrayItem` _team_resources (+ _index 3))))
      (bind _output_get_4 (set `local.F` _output_amount_4))
      (return _output_get _output_get_2 _output_get_3 _output_get_4))))

(fn `Modify Resource`
  (params (Resource :type "/Game/Blueprints/Core/Resources/Utilities/E_Resources Enum" :default "NewEnumerator3") (Amount :type Integer))
  (for _index (range (`KismetArrayLibrary.Array_Length` (`self.Team Resources`)))
    (bind (_output_player _output_resource) (break `/Game/Blueprints/Core/Resources/Utilities/S_TeamResources` (`|GetArrayItem` (`self.Team Resources`) _index)))
    (if (and (== (`self.CurrentPlayer`) _output_player) (`KismetStringLibrary.EqualEqual_StrStr` (`|GetEnumeratorNameAsString` (`local.Resource`)) (`|GetEnumeratorNameAsString` _output_resource)))
      (bind (_output_player_2 _output_resource_2 _output_amount) (break `/Game/Blueprints/Core/Resources/Utilities/S_TeamResources` (`|GetArrayItem` (`self.Team Resources`) _index)))
      (`KismetArrayLibrary.Array_Set` (`self.Team Resources`) _index (make `/Game/Blueprints/Core/Resources/Utilities/S_TeamResources` (`self.CurrentPlayer`) (`local.Resource`) (+ (`local.Amount`) _output_amount)))
      (break))))

(fn `Set Starting Resources`
  (params (Player :type Integer))
  (bind _returnvalue (`|GetDataTableRow` "/Game/Blueprints/Core/Resources/Utilities/DT_TeamResources.DT_TeamResources" "StartingGold")
    (:`then`
      (`KismetArrayLibrary.Array_Add` (`self.Team Resources`) (make `/Game/Blueprints/Core/Resources/Utilities/S_TeamResources` Player (`.Resource_28_D5A4197E4CB586921ACDF9B2E6806DBF` (break `/Game/Blueprints/Core/Resources/Utilities/S_TeamResources` _returnvalue)) (`.Amount_27_C21C821845B3CE6144AC84901EF39B77` (break `/Game/Blueprints/Core/Resources/Utilities/S_TeamResources` _returnvalue))))
      (bind _returnvalue_2 (`|GetDataTableRow` "/Game/Blueprints/Core/Resources/Utilities/DT_TeamResources.DT_TeamResources" "StartingWood")
        (:`then`
          (`KismetArrayLibrary.Array_Add` (`self.Team Resources`) (make `/Game/Blueprints/Core/Resources/Utilities/S_TeamResources` Player (`.Resource_28_D5A4197E4CB586921ACDF9B2E6806DBF` (break `/Game/Blueprints/Core/Resources/Utilities/S_TeamResources` _returnvalue_2)) (`.Amount_27_C21C821845B3CE6144AC84901EF39B77` (break `/Game/Blueprints/Core/Resources/Utilities/S_TeamResources` _returnvalue_2))))
          (bind _returnvalue_3 (`|GetDataTableRow` "/Game/Blueprints/Core/Resources/Utilities/DT_TeamResources.DT_TeamResources" "StartingStone")
            (:`then`
              (`KismetArrayLibrary.Array_Add` (`self.Team Resources`) (make `/Game/Blueprints/Core/Resources/Utilities/S_TeamResources` Player (`.Resource_28_D5A4197E4CB586921ACDF9B2E6806DBF` (break `/Game/Blueprints/Core/Resources/Utilities/S_TeamResources` _returnvalue_3)) (`.Amount_27_C21C821845B3CE6144AC84901EF39B77` (break `/Game/Blueprints/Core/Resources/Utilities/S_TeamResources` _returnvalue_3))))
              (bind _returnvalue_4 (`|GetDataTableRow` "/Game/Blueprints/Core/Resources/Utilities/DT_TeamResources.DT_TeamResources" "StartingFood")
                (:`then`
                  (`KismetArrayLibrary.Array_Add` (`self.Team Resources`) (make `/Game/Blueprints/Core/Resources/Utilities/S_TeamResources` Player (`.Resource_28_D5A4197E4CB586921ACDF9B2E6806DBF` (break `/Game/Blueprints/Core/Resources/Utilities/S_TeamResources` _returnvalue_4)) (`.Amount_27_C21C821845B3CE6144AC84901EF39B77` (break `/Game/Blueprints/Core/Resources/Utilities/S_TeamResources` _returnvalue_4)))))))))))))

(fn `UserConstructionScript`)