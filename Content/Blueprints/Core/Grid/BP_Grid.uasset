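; Hexagonal tile grid actor that builds a walkable map fitted to the level and maps cursor positions to tile indices.
; Construction script fills a tile map on parity-offset doubled-Y coordinates, using sphere traces to snap height and read BP_GridModifier types, keeping only walkable tiles.
; Tile and state edits are pushed to a child BP_GridVisual.
; Cursor picking tries two trace channels, then falls back to intersecting the grid plane.
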(event `self.ReceiveBeginPlay`)

(event `self.ReceiveTick`
  (params (DeltaSeconds :type "Float (single-precision)")))

(fn `AddGridTile`
  (params (Data :type "/Game/Blueprints/Core/Grid/Utilities/S_TileData Structure"))
  (bind _data_index (break `/Game/Blueprints/Core/Grid/Utilities/S_TileData` (`local.Data`)))
  (`BlueprintMapLibrary.Map_Add` (`self.GridTiles`) _data_index (`local.Data`))
  (`/Game/Blueprints/Core/Grid/BP_GridVisual.UpdateTilesVisual` (`self.Grid Visual`) (`local.Data`)))

(fn `AddStateToTile`
  (params (Index :type "IntPoint Structure") (State :type "/Game/Blueprints/Core/Grid/Utilities/E_TileState Enum" :default "NewEnumerator0"))
  (locals (Data :type "/Game/Blueprints/Core/Grid/Utilities/S_TileData Structure"))
  (bind _data_index (break `/Game/Blueprints/Core/Grid/Utilities/S_TileData` (`local.Data`)))
  (bind (_value _returnvalue) (`BlueprintMapLibrary.Map_Find` (`self.GridTiles`) Index))
  (if _returnvalue
    (bind _output_get (set `local.Data` _value))
    (bind _returnvalue_2 (`KismetArrayLibrary.Array_AddUnique` (`.States_12_361B67934D09680D08838496024BC194` (break `/Game/Blueprints/Core/Grid/Utilities/S_TileData` _output_get)) State))
    (if (>= _returnvalue_2 0)
      (`BlueprintMapLibrary.Map_Add` (`self.GridTiles`) _data_index (`local.Data`))
      (`/Game/Blueprints/Core/Grid/BP_GridVisual.UpdateTilesVisual` (`self.Grid Visual`) (`local.Data`)))))

(fn `CalculateCenterAndBottomLeft`
  (returns (Center :type "Vector Structure") (BottomLeft :type "Vector Structure"))
  (locals (C :type "Vector Structure" :default (0.0 0.0 0.0)))
  (bind (_tile_count_x _tile_count_y) (break `IntPoint` (`self.Tile Count`)))
  (set `local.C` (`/Game/Blueprints/Core/Utilities/BFL_Utilities.SnapVectorToVector` (`self.Center Location`) (* (`self.Tile Size`) (0.75 0.5 0.0))))
  (return (`local.C`) (- (`local.C`) (* (/ (- (`self.Tile Count`) (`KismetMathLibrary.MakeVector2D` (`KismetMathLibrary.SelectFloat` 0.0 1.0 (`/Game/Blueprints/Core/Utilities/BFL_Utilities.IsIntEven` _tile_count_x)) (`KismetMathLibrary.SelectFloat` 0.0 1.0 (`/Game/Blueprints/Core/Utilities/BFL_Utilities.IsIntEven` _tile_count_y)))) 2.0) (`KismetMathLibrary.Conv_VectorToVector2D` (`self.Tile Size`))))))

(fn `DestroyGrid`
  (`BlueprintMapLibrary.Map_Clear` (`self.GridTiles`))
  (`/Game/Blueprints/Core/Grid/BP_GridVisual.DestroyGridVisual` (`self.Grid Visual`)))

(fn `GetCurrentShapeData`
  (returns (ReturnValue :type "/Game/Blueprints/Core/Grid/GridShapes/S_GridShapeData Structure"))
  (return (`/Game/Blueprints/Core/Grid/GridShapes/BFL_GridShape.GetShapeData` (`self.Shape`))))

(fn `GetCursorLocationOnGrid`
  (params (PlayerIndex :type Integer))
  (returns (Location :type "Vector Structure"))
  (bind _returnvalue (`GameplayStatics.GetPlayerController` PlayerIndex))
  (bind (_hitresult _returnvalue_2) (`PlayerController.GetHitResultUnderCursorByChannel` _returnvalue "TraceTypeQuery4" false))
  (bind (_hitresult_2 _returnvalue_3) (`PlayerController.GetHitResultUnderCursorByChannel` _returnvalue "TraceTypeQuery3" false))
  (bind (_worldlocation _worlddirection) (`PlayerController.DeprojectMousePositionToWorld` _returnvalue))
  (bind (_t _intersection _returnvalue_4) (`KismetMathLibrary.LinePlaneIntersection` _worldlocation (+ _worldlocation (* _worlddirection 99999999999999.0)) (`KismetMathLibrary.MakePlaneFromPointAndNormal` (`self.Center Location`) (0.0 0.0 1.0))))
  (if _returnvalue_2
    (return (`.Location` (`GameplayStatics.BreakHitResult` _hitresult)))
    (elif _returnvalue_3
      (return (`.Location` (`GameplayStatics.BreakHitResult` _hitresult_2)))
      (elif _returnvalue_4
        (return _intersection)
        (else
          (return (-999.0 -999.0 -999.0)))))))

(fn `GetTileIndexUnderCursor`
  (params (PlayerIndex :type Integer))
  (returns (Index :type "IntPoint Structure"))
  (bind _location (`self.GetCursorLocationOnGrid` PlayerIndex))
  (bind _index (`self.GetTileLocationFromWorldLocation` _location))
  (return _index))

(fn `GetTileLocationFromIndex`
  (params (Index :type "IntPoint Structure"))
  (returns (ReturnValue :type "Vector Structure"))
  (return (+ (`self.BottomLeftCornerLocation`) (* (`self.Tile Size`) (* Index (0.75 0.5))))))

(fn `GetTileLocationFromWorldLocation`
  (params (Location :type "Vector Structure"))
  (returns (Index :type "IntPoint Structure"))
  (locals (SnappedLocationOnGrid :type "IntPoint Structure") (LocationOnGrid :type "Vector Structure") (TempIndex :type "Vector2D Structure"))
  (bind _tempindex_x (`KismetMathLibrary.BreakVector2D` (`local.TempIndex`)))
  (bind (_tempindex_x_2 _tempindex_y) (`KismetMathLibrary.BreakVector2D` (`local.TempIndex`)))
  (bind (_tempindex_x_3 _tempindex_y_2) (`KismetMathLibrary.BreakVector2D` (`local.TempIndex`)))
  (set `local.LocationOnGrid` (- Location (`self.BottomLeftCornerLocation`)))
  (switch `/Game/Blueprints/Core/Grid/GridShapes/E_GridShape` (`self.Shape`)
    (:`NewEnumerator1`
      (return (make `IntPoint` -999 -999)))
    (:`NewEnumerator0`
      (set `local.SnappedLocationOnGrid` (`KismetMathLibrary.Conv_Vector2DToIntPoint` (`KismetMathLibrary.Conv_VectorToVector2D` (`/Game/Blueprints/Core/Utilities/BFL_Utilities.SnapVectorToVector` (* (`local.LocationOnGrid`) (1.0 2.0 1.0)) (* (`self.Tile Size`) (0.75 0.25 1.0))))))
      (set `local.TempIndex` (/ (`local.SnappedLocationOnGrid`) (* (`KismetMathLibrary.Conv_VectorToVector2D` (`self.Tile Size`)) (0.74 1.0))))
      (if (`/Game/Blueprints/Core/Utilities/BFL_Utilities.IsFloatEven` _tempindex_x)
        (return (make `IntPoint` (`KismetMathLibrary.FTrunc` _tempindex_x_2) (`KismetMathLibrary.FTrunc` (`KismetMathLibrary.Conv_IntToDouble` (* (`KismetMathLibrary.Round` (/ _tempindex_y 2.0)) 2)))))
        (else
          (return (make `IntPoint` (`KismetMathLibrary.FTrunc` _tempindex_x_3) (`KismetMathLibrary.FTrunc` (`KismetMathLibrary.Conv_IntToDouble` (+ (* (`KismetMathLibrary.FFloor` (/ _tempindex_y_2 2.0)) 2) 1))))))))))

(fn `GetTileScale`
  (returns (ReturnValue :type "Vector Structure"))
  (return (/ (`self.Tile Size`) (`.MeshSize_2_03CF4F614C6324128B3DAE8CA0698EB8` (break `/Game/Blueprints/Core/Grid/GridShapes/S_GridShapeData` (`self.GetCurrentShapeData`))))))

(fn `IsIndexValid`
  (params (Index :type "IntPoint Structure"))
  (returns (IsValid :type Boolean))
  (return (`BlueprintMapLibrary.Map_Contains` (`self.GridTiles`) Index)))

(fn `RemoveGridTile`
  (params (Index :type "IntPoint Structure"))
  (bind _returnvalue (`BlueprintMapLibrary.Map_Remove` (`self.GridTiles`) Index))
  (if _returnvalue
    (`/Game/Blueprints/Core/Grid/BP_GridVisual.UpdateTilesVisual` (`self.Grid Visual`) (make `/Game/Blueprints/Core/Grid/Utilities/S_TileData` (`local.Index`)))))

(fn `RemoveStateToTile`
  (params (Index :type "IntPoint Structure") (State :type "/Game/Blueprints/Core/Grid/Utilities/E_TileState Enum" :default "NewEnumerator0"))
  (locals (Data :type "/Game/Blueprints/Core/Grid/Utilities/S_TileData Structure"))
  (bind _data_index (break `/Game/Blueprints/Core/Grid/Utilities/S_TileData` (`local.Data`)))
  (bind (_value _returnvalue) (`BlueprintMapLibrary.Map_Find` (`self.GridTiles`) Index))
  (if _returnvalue
    (bind _output_get (set `local.Data` _value))
    (`KismetArrayLibrary.Array_RemoveItem` (`.States_12_361B67934D09680D08838496024BC194` (break `/Game/Blueprints/Core/Grid/Utilities/S_TileData` _output_get)) State)
    (if true
      (`BlueprintMapLibrary.Map_Add` (`self.GridTiles`) _data_index (`local.Data`))
      (`/Game/Blueprints/Core/Grid/BP_GridVisual.UpdateTilesVisual` (`self.Grid Visual`) (`local.Data`)))))

(fn `SpawnGrid`
  (params (CenterLocation :type "Vector Structure") (TileSize :type "Vector Structure") (TileCount :type "IntPoint Structure") (Shape :type "/Game/Blueprints/Core/Grid/GridShapes/E_GridShape Enum" :default "NewEnumerator1") (UseEnviroment :type Boolean))
  (locals (X :type Integer) (Y :type Integer) (TileTransform :type "Transform Structure") (Index :type "IntPoint Structure"))
  (bind (_tile_count_x _tile_count_y) (break `IntPoint` (`self.Tile Count`)))
  (bind (_tiletransform_location _tiletransform_rotation _tiletransform_scale) (`KismetMathLibrary.BreakTransform` (`local.TileTransform`)))
  (bind _tile_count_x_2 (break `IntPoint` (`self.Tile Count`)))
  (set `self.Center Location` CenterLocation)
  (set `self.Tile Size` TileSize)
  (set `self.Tile Count` TileCount)
  (set `self.Shape` Shape)
  (`self.DestroyGrid`)
  (`/Game/Blueprints/Core/Grid/BP_GridVisual.Initialize Grid Visual` (`self.Grid Visual`) self)
  (bind (_center _bottomleft) (`self.CalculateCenterAndBottomLeft`))
  (set `self.Center Location` _center)
  (set `self.BottomLeftCornerLocation` _bottomleft)
  (for _index (range _tile_count_x_2)
    (set `local.X` _index)
    (for _index_2 (range (`KismetMathLibrary.SelectInt` 0 1 (`/Game/Blueprints/Core/Utilities/BFL_Utilities.IsIntEven` (`local.X`))) (* _tile_count_y 2))
      (set `local.Y` _index_2)
      (`|ExecutionSequence`
        (:`then_0`
          (set `local.Index` (make `IntPoint` (`local.X`) (`local.Y`)))
          (set `local.TileTransform` (`KismetMathLibrary.MakeTransform` (`self.GetTileLocationFromIndex` (`local.Index`)) (struct) (`self.GetTileScale`)))
          (if (`local.UseEnviroment`)
            (bind (_outlocation _tiletype) (`self.TraceForGround` _tiletransform_location))
            (if (`/Game/Blueprints/Core/Grid/Utilities/BFL_TileData.IsTileTypeWalkable` _tiletype)
              (`self.AddGridTile` (make `/Game/Blueprints/Core/Grid/Utilities/S_TileData` (`local.Index`) _tiletype (`KismetMathLibrary.MakeTransform` _outlocation _tiletransform_rotation _tiletransform_scale))))))
        (:`then_1`
          (`/Engine/EditorBlueprintResources/StandardMacros.IncrementInt` _index_2))))))

(fn `TraceForGround`
  (params (TileLocation :type "Vector Structure"))
  (returns (OutLocation :type "Vector Structure") (TileType :type "/Game/Blueprints/Core/Grid/Utilities/E_TileType Enum"))
  (locals (RedType :type "/Game/Blueprints/Core/Grid/Utilities/E_TileType Enum" :default "NewEnumerator0") (RedZ :type "Float (double-precision)" :default 0.0))
  (bind _tile_size_x (`KismetMathLibrary.BreakVector` (`self.Tile Size`)))
  (bind (_tilelocation_x _tilelocation_y) (`KismetMathLibrary.BreakVector` (`local.TileLocation`)))
  (bind (_tile_size_x_2 _tile_size_y _tile_size_z) (`KismetMathLibrary.BreakVector` (`self.Tile Size`)))
  (set `self.Radius` (/ _tile_size_x 5.0))
  (bind _outhits (`KismetSystemLibrary.SphereTraceMulti` (+ (`local.TileLocation`) (0.0 0.0 1000.0)) (- (`local.TileLocation`) (0.0 0.0 1000.0)) (`self.Radius`) "TraceTypeQuery3"))
  (if (> (`KismetArrayLibrary.Array_Length` _outhits) 0)
    (set `local.RedType` "NewEnumerator1")
    (for _array_element _outhits
      (bind (_bblockinghit _binitialoverlap _time _distance _location _impactpoint _normal _impactnormal _physmat _hitactor) (`GameplayStatics.BreakHitResult` _array_element))
      (bind _asbp_grid_modifier (cast `/Game/Blueprints/Core/Grid/Utilities/BP_GridModifier` _hitactor)
        (:`then`
          (set `local.RedType` (`/Game/Blueprints/Core/Grid/Utilities/BP_GridModifier.Type` _asbp_grid_modifier)))
        (:`CastFailed`
          _))
      (set `local.RedZ` (`KismetMathLibrary.GridSnap_Float` (- (.z _location) (`self.Radius`)) _tile_size_z)))
    (return (`KismetMathLibrary.MakeVector` _tilelocation_x _tilelocation_y (`local.RedZ`)) (`local.RedType`))
    (else
      (return (`local.TileLocation`) "NewEnumerator0"))))

(fn `UserConstructionScript`
  (set `self.Grid Visual` (cast `/Game/Blueprints/Core/Grid/BP_GridVisual` (`ChildActorComponent.ChildActor` (`self.ChildActor_GridVisual`)) :!pure true))
  (`self.SpawnGrid` (`self.K2_GetActorLocation`) (`self.Tile Size`) (`self.Tile Count`) (`self.Shape`) true))