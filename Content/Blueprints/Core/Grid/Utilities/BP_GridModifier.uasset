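; BP_GridModifier is a grid utility actor, hidden in game, that carries a tile Type such as obstacle, movement cost or flying-only.
; Its construction script applies the flat hexagon grid material and tints it by Type as a color-coded marker.
; The same script sets the mesh to overlap one custom trace channel and block another, with no active runtime logic.
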(fn `UserConstructionScript`
  (bind _staticmesh (`self.StaticMesh`))
  (bind _staticmesh_2 (`self.StaticMesh`))
  (`PrimitiveComponent.SetMaterial` _staticmesh_2 0 "/Game/Blueprints/Core/Grid/Hexagon/MI_Grid_Flat_Hexagon.MI_Grid_Flat_Hexagon")
  (`MeshComponent.SetVectorParameterValueOnMaterials` _staticmesh_2 "Color" (`KismetMathLibrary.Conv_LinearColorToVector` (select `/Game/Blueprints/Core/Grid/Utilities/E_TileType` (`self.Type`) :`NewEnumerator1` (struct :`R` 1.0 :`G` 1.0 :`B` 1.0 :`A` 1.0) :`NewEnumerator2` (struct :`R` 1.0 :`B` 0.068094 :`A` 1.0) :`NewEnumerator3` (struct :`R` 0.871018 :`G` 1.0 :`B` 0.069587 :`A` 1.0) :`NewEnumerator4` (struct :`R` 1.0 :`G` 0.594607 :`A` 1.0) :`NewEnumerator5` (struct :`R` 0.997782 :`B` 1.0 :`A` 1.0) :!type "LinearColor Structure")))
  (`PrimitiveComponent.SetCollisionResponseToChannel` _staticmesh "ECC_GameTraceChannel1" "ECR_Overlap")
  (`PrimitiveComponent.SetCollisionResponseToChannel` _staticmesh "ECC_GameTraceChannel4" "ECR_Block")
  (`self.SetActorHiddenInGame` true))