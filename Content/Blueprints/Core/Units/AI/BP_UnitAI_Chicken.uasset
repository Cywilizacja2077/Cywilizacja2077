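; AI for the Chicken combat unit, extending a parent unit AI to treat one specific spell as a self-cast fallback.
; The spell is removed from the parent's available spell list, keeping it out of that pool.
; When spell selection finishes without a valid choice, the unit casts it on itself if CanCastSpell passes, then hands off to the parent's completion logic.
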(event `self.DecideWhichSpellToCast_Done`
  (bind _index (`/Game/Blueprints/Core/Units/BP_Unit.Index` (`self.Unit`)))
  (`|ExecutionSequence`
    (:`then_0`
      (if (not (`.IsSpellValid_1_1A9A43124E397150990AF284FF973DFE` (break `/Game/Blueprints/Core/Units/AI/S_UnitAISpellCastingData` (`self.AISpellCasting`))))
        (bind _spelldata (`/Game/Blueprints/Core/Combat/Spells/Utilities/BFL_Spells.Get Spell Data from Spell` "NewEnumerator10"))
        (bind _cancast (`/Game/Blueprints/Core/Units/BP_Unit.CanCastSpell` (`self.Unit`) _spelldata (`/Game/Blueprints/Core/Combat/BP_CombatSystem.Resources Ref` (`self.CombatSystem`))))
        (if _cancast
          (set `self.AISpellCasting` (make `/Game/Blueprints/Core/Units/AI/S_UnitAISpellCastingData` true "NewEnumerator10" _index _index)))))
    (:`then_1`
      (`parent.DecideWhichSpellToCast_Done`))))

(fn `GetAvaliableSpells`
  (returns (AvaliableSpells :type "Array of /Game/Blueprints/Core/Combat/Spells/Utilities/E_Spell Enum"))
  (locals (Ret :type "Array of /Game/Blueprints/Core/Combat/Spells/Utilities/E_Spell Enum"))
  (bind _output_get (set `local.Ret` (`parent.GetAvaliableSpells`)))
  (`KismetArrayLibrary.Array_RemoveItem` _output_get "NewEnumerator10")
  (return (`local.Ret`)))

(fn `UserConstructionScript`
  (`parent.UserConstructionScript`))