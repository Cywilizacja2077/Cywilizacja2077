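; Ranger-specific unit AI Blueprint that varies its combat movement logic by turn parity and whether it has cast a damaging spell.
; A turn counter resets at combat start and increments each AI turn, which also clears the damage flag.
; Casting a spell with a negative minimum HP modifier sets that flag.
; GetUnitMovementLogic returns one mode on even turns without damage and another otherwise.
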(event `self.CastSpell`
  (bind _spelldata (`/Game/Blueprints/Core/Combat/Spells/Utilities/BFL_Spells.Get Spell Data from Spell` (`.Spell_4_4D6D3BE74B8D414C94FE71A963252D68` (break `/Game/Blueprints/Core/Units/AI/S_UnitAISpellCastingData` (`self.AISpellCasting`)))))
  (set `self.DamageAtUnitThisTurn` (or (`self.DamageAtUnitThisTurn`) (< (`.X` (break `IntPoint` (`.MinMaxModfierHP_3_F7181E8446E84D66A7579AB5FE7C4F63` (break `/Game/Blueprints/Core/Combat/Spells/Utilities/S_SpellData_Impact` (`.Impact_18_0B1574FF4667A534735DD69CB45358B7` (break `/Game/Blueprints/Core/Combat/Spells/Utilities/S_SpellData` _spelldata)))))) 0)))
  (`parent.CastSpell`))

(fn `AICombatEnded`
  (`parent.AICombatEnded`))

(fn `AICombatStarted`
  (set `self.TurnCount` 0)
  (`parent.AICombatStarted`))

(fn `AIPlayTurn`
  (`/Engine/EditorBlueprintResources/StandardMacros.IncrementInt` (`self.TurnCount`)
    (:`  `
      (set `self.DamageAtUnitThisTurn` false)
      (`parent.AIPlayTurn`))))

(fn `GetUnitMovementLogic`
  (returns (MovementLogic :type "/Game/Blueprints/Core/Units/AI/E_UnitAIMovementLogic Enum"))
  (return (select `bool` (and (`/Game/Blueprints/Core/Utilities/BFL_Utilities.IsIntEven` (`self.TurnCount`)) (not (`self.DamageAtUnitThisTurn`))) :`false` "NewEnumerator2" :`true` "NewEnumerator0" :!type "/Game/Blueprints/Core/Units/AI/E_UnitAIMovementLogic Enum")))

(fn `UserConstructionScript`
  (`parent.UserConstructionScript`))