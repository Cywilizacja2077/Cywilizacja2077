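; Player camera pawn that pans and zooms a spring-arm view and owns the main HUD with its context menu.
; Enhanced Input actions set a desired location and a clamped zoom, which Tick interpolates toward for smooth movement.
; It creates the HUD on BeginPlay; the context-menu action stores the mouse position and cursor hit before opening the menu, and tile selection closes it.
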(event `EnhancedInput|/Game/Blueprints/Core/Input/Actions/Open_Context_Menu`
  (params (ActionValue :type Boolean) (ElapsedSeconds :type "Float (double-precision)") (TriggeredSeconds :type "Float (double-precision)") (InputAction :type "InputAction Object Reference" :default "/Game/Blueprints/Core/Input/Actions/Open_Context_Menu.Open_Context_Menu"))
  (:`Triggered`
    (`self.Create Context Menu`)))

(event `EnhancedInput|/Game/Blueprints/Core/Input/Actions/Select_Tile`
  (params (ActionValue :type Boolean) (ElapsedSeconds :type "Float (double-precision)") (TriggeredSeconds :type "Float (double-precision)") (InputAction :type "InputAction Object Reference" :default "/Game/Blueprints/Core/Input/Actions/Select_Tile.Select_Tile"))
  (:`Triggered`
    (`/Game/Blueprints/HUD/MainHUD.Close Context` (`self.Main HUD Ref`))))

(event `self.ReceiveBeginPlay`
  (bind _asplayer_controller (cast `PlayerController` (`self.GetController`)))
  (`EnhancedInputSubsystemInterface.AddMappingContext` (pcsubsystem `EnhancedInputLocalPlayerSubsystem` _asplayer_controller) "/Game/Blueprints/Core/Input/DefaultInputForPC.DefaultInputForPC" 0 (struct))
  (set `self.Location_Desired` (`self.K2_GetActorLocation`))
  (set `self.Zoom_Desired` (`SpringArmComponent.TargetArmLength` (`self.SpringArm`)))
  (`self.Create Main HUD`))

(event `EnhancedInput|/Game/Blueprints/Core/Input/Actions/Action_Move`
  (params (ActionValue :type "Vector2D Structure") (ElapsedSeconds :type "Float (double-precision)") (TriggeredSeconds :type "Float (double-precision)") (InputAction :type "InputAction Object Reference" :default "/Game/Blueprints/Core/Input/Actions/Action_Move.Action_Move"))
  (bind (_x _y) (`KismetMathLibrary.BreakVector2D` ActionValue))
  (:`Triggered`
    (set `self.Location_Desired` (+ (* (`self.GetActorForwardVector`) (* (`self.Location_Speed`) _x)) (`self.Location_Desired`) (* (* _y (`self.Location_Speed`)) (`self.GetActorRightVector`))))))

(event `EnhancedInput|/Game/Blueprints/Core/Input/Actions/Action_Zoom`
  (params (ActionValue :type "Float (double-precision)") (ElapsedSeconds :type "Float (double-precision)") (TriggeredSeconds :type "Float (double-precision)") (InputAction :type "InputAction Object Reference" :default "/Game/Blueprints/Core/Input/Actions/Action_Zoom.Action_Zoom"))
  (:`Triggered`
    (set `self.Zoom_Desired` (`KismetMathLibrary.FClamp` (+ (`self.Zoom_Desired`) (* ActionValue (`self.Zoom_Speed`))) (`self.Zoom_Min`) (`self.Zoom_Max`)))))

(event `self.ReceiveTick`
  (params (DeltaSeconds :type "Float (single-precision)"))
  (bind _springarm (`self.SpringArm`))
  (set `SpringArmComponent.TargetArmLength` (`KismetMathLibrary.FInterpTo` (`SpringArmComponent.TargetArmLength` _springarm) (`self.Zoom_Desired`) DeltaSeconds (`self.Zoom_Interp`)) _springarm)
  (`self.K2_SetActorLocation` (`KismetMathLibrary.VInterpTo` (`self.K2_GetActorLocation`) (`self.Location_Desired`) DeltaSeconds (`self.Location_Interp`))))

(fn `Create Context Menu`
  (bind (_locationx _locationy) (`PlayerController.GetMousePosition` (`GameplayStatics.GetPlayerController` 0)))
  (set `self.Mouse Position` (`KismetMathLibrary.MakeVector` _locationx _locationy))
  (set `self.Mouse Hit Result` (`PlayerController.GetHitResultUnderCursorByChannel` (`GameplayStatics.GetPlayerController` 0) "TraceTypeQuery1" true))
  (`/Game/Blueprints/HUD/MainHUD.Open Context` (`self.Main HUD Ref`)))

(fn `Create Main HUD`
  (bind _returnvalue (`|CreateWidget` "/Game/Blueprints/HUD/MainHUD.MainHUD_C" (`GameplayStatics.GetPlayerController` 0)))
  (bind _output_get (set `self.Main HUD Ref` _returnvalue))
  (`UserWidget.AddToViewport` _output_get 0))

(fn `UserConstructionScript`)