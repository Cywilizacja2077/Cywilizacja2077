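; BP_PlayerActions is the player input actor that turns mouse hovering and clicks on BP_Grid into tile actions.
; Each tick it finds the tile under the cursor, moves a hover state onto it and fires OnHoverTileChanged.
; Left and right buttons each execute a spawned, swappable action actor on press and again on each new tile while held, allowing drag application.
; Both buttons start with Action_SelectTile.
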(event `self.ReceiveBeginPlay`
  (bind _returnvalue (`GameplayStatics.GetActorOfClass` "/Game/Blueprints/Core/Grid/BP_Grid.BP_Grid_C"))
  (set `self.Grid` _returnvalue)
  (`self.EnableInput` (`GameplayStatics.GetPlayerController` 0))
  (`self.SetSelectedAction` "/Game/Blueprints/Core/Player/Actions/Grid/Action_SelectTile.Action_SelectTile_C" "/Game/Blueprints/Core/Player/Actions/Grid/Action_SelectTile.Action_SelectTile_C"))

(event `self.ReceiveTick`
  (params (DeltaSeconds :type "Float (single-precision)"))
  (`self.UpdateTileHovered`))

(event `Key|LeftMouseButton`
  (params (Key :type "Key Structure"))
  (:`Pressed`
    (`self.UpdateTileHovered`)
    (set `self.IsLeftClickDown` true)
    (`/Engine/EditorBlueprintResources/StandardMacros.IsValid` (`self.SelectedAction_LeftClick`) :!label _label
      (:`Is Valid`
        (`/Game/Blueprints/Core/Player/Actions/BP_Action.ExecuteAction` (`self.SelectedAction_LeftClick`) (`self.HoverTile`)))))
  (:`Released`
    (set `self.IsLeftClickDown` false)))

(event `OnHoverTileChanged`
  (`|ExecutionSequence`
    (:`then_0`
      (if (`self.IsLeftClickDown`)
        (goto _label)))
    (:`then_1`
      (if (`self.IsRightClickDown`)
        (`/Engine/EditorBlueprintResources/StandardMacros.IsValid` (`self.SelectedAction_RightClick`) :!label _label_2
          (:`Is Valid`
            (`/Game/Blueprints/Core/Player/Actions/BP_Action.ExecuteAction` (`self.SelectedAction_RightClick`) (`self.HoverTile`))))))))

(event `Key|RightMouseButton`
  (params (Key :type "Key Structure"))
  (:`Pressed`
    (`self.UpdateTileHovered`)
    (set `self.IsRightClickDown` true)
    (goto _label_2))
  (:`Released`
    (set `self.IsRightClickDown` false)))

(fn `SetSelectedAction`
  (params (LeftAction :type "/Game/Blueprints/Core/Player/Actions/BP_Action Class Reference") (RightAction :type "/Game/Blueprints/Core/Player/Actions/BP_Action Class Reference"))
  (bind _selectedaction_rightclick (`self.SelectedAction_RightClick`))
  (bind _selectedaction_leftclick (`self.SelectedAction_LeftClick`))
  (`|ExecutionSequence`
    (:`then_0`
      (`/Engine/EditorBlueprintResources/StandardMacros.IsValid` _selectedaction_leftclick
        (:`Is Valid`
          (`self.K2_DestroyActor` _selectedaction_leftclick)
          (set `self.SelectedAction_LeftClick` null))
        (:`Is Not Valid`
          _))
      (if (`KismetSystemLibrary.IsValidClass` (`local.LeftAction`))
        (bind _returnvalue (`|SpawnActorFromClass` (`local.LeftAction`) (`KismetMathLibrary.MakeTransform` (0.0 0.0 0.0)) "AlwaysSpawn" "MultiplyWithRoot" null self null))
        (set `self.SelectedAction_LeftClick` _returnvalue)))
    (:`then_1`
      (`/Engine/EditorBlueprintResources/StandardMacros.IsValid` _selectedaction_rightclick
        (:`Is Valid`
          (`self.K2_DestroyActor` _selectedaction_rightclick)
          (set `self.SelectedAction_RightClick` null))
        (:`Is Not Valid`
          _))
      (if (`KismetSystemLibrary.IsValidClass` (`local.RightAction`))
        (bind _returnvalue_2 (`|SpawnActorFromClass` (`local.RightAction`) (`KismetMathLibrary.MakeTransform` (0.0 0.0 0.0)) "AlwaysSpawn" "MultiplyWithRoot" null self null))
        (set `self.SelectedAction_RightClick` _returnvalue_2)))))

(fn `UpdateTileHovered`
  (bind _index (`/Game/Blueprints/Core/Grid/BP_Grid.GetTileIndexUnderCursor` (`self.Grid`) 0))
  (if (!= _index (`self.HoverTile`))
    (`/Game/Blueprints/Core/Grid/BP_Grid.RemoveStateToTile` (`self.Grid`) (`self.HoverTile`) "NewEnumerator1")
    (set `self.HoverTile` _index)
    (`/Game/Blueprints/Core/Grid/BP_Grid.AddStateToTile` (`self.Grid`) (`self.HoverTile`) "NewEnumerator1")
    (`self.OnHoverTileChanged`)))

(fn `UserConstructionScript`)