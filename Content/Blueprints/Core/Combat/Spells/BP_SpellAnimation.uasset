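; BP_SpellAnimation is an actor that plays a spell's visual effect on the grid, then destroys itself.
; On BeginPlay it spawns a BP_AnimatedShape hexagon for each attacked tile, animating from a tiny shape at the origin tile to that tile's transform, with randomized brightness and play rate.
; Only the first shape's completion is bound, so it alone triggers the OnSpellAnimationCompleted dispatcher and the actor's destruction, even if other shapes are still animating.
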(event `self.ReceiveBeginPlay`
  (`self.Event_PlaySpellAnimation`))

(event `Event_PlaySpellAnimation`
  (bind (_transform_location _transform_rotation) (`KismetMathLibrary.BreakTransform` (`self.GetTileTrasform` (`self.OriginIndex`))))
  (for (_array_element _array_index) (`self.AttackedIndexes`)
    (bind _returnvalue (`|SpawnActorFromClass` "/Game/Blueprints/Core/Combat/Spells/SpellAnimations/Components/BP_AnimatedShape.BP_AnimatedShape_C" (`KismetMathLibrary.MakeTransform` (0.0 0.0 0.0)) "AlwaysSpawn" "MultiplyWithRoot" null "/Game/Blueprints/Core/Grid/Hexagon/SM_Grid_Hexagon.SM_Grid_Hexagon" "/Engine/VREditor/BasicMeshes/MI_Cube_03.MI_Cube_03" (* (struct :`R` 1.0 :`B` 0.406657 :`A` 1.0) (`KismetMathLibrary.RandomFloatInRange` 0.5 1.5)) (`KismetMathLibrary.MakeTransform` _transform_location _transform_rotation (0.01 0.01 0.01)) (`self.GetTileTrasform` _array_element) (`KismetMathLibrary.RandomFloatInRange` 1.0 2.0) null))
    (if (== _array_index 0)
      (add `/Game/Blueprints/Core/Combat/Spells/SpellAnimations/Components/BP_AnimatedShape.OnShapeAnimationCompleted` _returnvalue (delegate `OnShapeAnimationCompleted`)))))

(event `OnShapeAnimationCompleted`
  (params (AnimatedShape :type "/Game/Blueprints/Core/Combat/Spells/SpellAnimations/Components/BP_AnimatedShape Object Reference"))
  (`self.Event_CompleteSpellAnimation`))

(event `Event_CompleteSpellAnimation`
  (`self.OnSpellAnimationCompleted` self)
  (`self.K2_DestroyActor`))

(fn `GetTileTrasform`
  (params (Index :type "IntPoint Structure (by ref)"))
  (returns (Transform :type "Transform Structure"))
  (return (`.Transform_8_8EB76CFC4BC00F30091A1E93DE74858B` (break `/Game/Blueprints/Core/Grid/Utilities/S_TileData` (`BlueprintMapLibrary.Map_Find` (`/Game/Blueprints/Core/Grid/BP_Grid.GridTiles` (`self.Grid`)) Index)))))

(fn `UserConstructionScript`)