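; Spell animation for Wind Gust that hits the target tile after a brief delay, then sends animated gusts out to the other attacked tiles.
; Each spawned BP_AnimatedWindGust grows from the target toward its tile at a random play rate.
; The completion handler reports that tile's hit and ends the spell when no indexes remain.
; A DoOnce inside the loop gates the completion binding, so only the first gust gets bound.
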(event `self.Event_PlaySpellAnimation`
  (bind _transform_location (`KismetMathLibrary.BreakTransform` (`self.GetTileTrasform` (`self.TargetIndex`))))
  (`KismetSystemLibrary.Delay` 0.1)
  (`self.OnAnimationHitTile` self (`self.TargetIndex`))
  (`KismetArrayLibrary.Array_RemoveItem` (`self.AttackedIndexes`) (`self.TargetIndex`))
  (for _array_element (`self.AttackedIndexes`)
    (bind _transform_location_2 (`KismetMathLibrary.BreakTransform` (`self.GetTileTrasform` _array_element)))
    (bind _returnvalue (`KismetMathLibrary.FindLookAtRotation` _transform_location _transform_location_2))
    (bind _returnvalue_2 (`|SpawnActorFromClass` "/Game/Blueprints/Core/Combat/Spells/SpellAnimations/Components/BP_AnimatedWindGust.BP_AnimatedWindGust_C" (`KismetMathLibrary.MakeTransform` (0.0 0.0 0.0)) "Undefined" "MultiplyWithRoot" null (`KismetMathLibrary.MakeTransform` _transform_location _returnvalue (0.1 0.1 0.1)) (`KismetMathLibrary.MakeTransform` _transform_location_2 _returnvalue (0.3 0.3 0.3)) (`KismetMathLibrary.RandomFloatInRange` 0.5 1.5) _array_element null))
    (`/Engine/EditorBlueprintResources/StandardMacros.DoOnce` false
      (:`Completed`
        (add `/Game/Blueprints/Core/Combat/Spells/SpellAnimations/Components/BP_AnimatedWindGust.OnShapeAnimationCompleted` _returnvalue_2 (delegate `OnAnimationCompletedd`))))))

(event `OnAnimationCompletedd`
  (params (AnimatedShape :type "/Game/Blueprints/Core/Combat/Spells/SpellAnimations/Components/BP_AnimatedWindGust Object Reference"))
  (bind _index (`/Game/Blueprints/Core/Combat/Spells/SpellAnimations/Components/BP_AnimatedWindGust.Index` AnimatedShape))
  (bind _attackedindexes (`self.AttackedIndexes`))
  (`self.OnAnimationHitTile` self _index)
  (`KismetArrayLibrary.Array_RemoveItem` _attackedindexes _index)
  (if (== (`KismetArrayLibrary.Array_Length` _attackedindexes) 0)
    (`self.Event_CompleteSpellAnimation`)))

(fn `UserConstructionScript`
  (`parent.UserConstructionScript`))