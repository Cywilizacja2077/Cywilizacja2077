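; BP_SpellAnim_Heal is the visual animation for the Heal spell, played on a target tile.
; The play event moves the actor to that tile and runs a timeline that rotates and scales the AnimRotationScale component while driving material opacity on three static meshes.
; When the timeline finishes, it signals that the spell animation is complete.
; The construction script tints each mesh a different shade of green.
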(event `self.Event_PlaySpellAnimation`
  (bind _transform_location (`KismetMathLibrary.BreakTransform` (`self.GetTileTrasform` (`self.TargetIndex`))))
  (`self.K2_SetActorLocation` _transform_location)
  (bind (_direction _opacity _scale _rotation) (`Timeline|Timeline` :!via `PlayFromStart`)
    (:`Update`
      (`SceneComponent.K2_SetRelativeRotation` (`self.Anim_RotationScale`) (`KismetMathLibrary.MakeRotator` 0.0 0.0 _rotation) false false)
      (`SceneComponent.SetRelativeScale3D` (`self.Anim_RotationScale`) _scale)
      (`MeshComponent.SetScalarParameterValueOnMaterials` (`self.StaticMesh2`) "Opacity" _opacity)
      (`MeshComponent.SetScalarParameterValueOnMaterials` (`self.StaticMesh1`) "Opacity" _opacity)
      (`MeshComponent.SetScalarParameterValueOnMaterials` (`self.StaticMesh`) "Opacity" _opacity)
      (`MeshComponent.SetScalarParameterValueOnMaterials` (`self.StaticMesh+`) "Opacity" _opacity)
      (`MeshComponent.SetScalarParameterValueOnMaterials` (`self.StaticMesh+1`) "Opacity" _opacity)
      (`MeshComponent.SetScalarParameterValueOnMaterials` (`self.StaticMesh+2`) "Opacity" _opacity))
    (:`Finished`
      (`self.Event_CompleteSpellAnimation`))))

(fn `UserConstructionScript`
  (`parent.UserConstructionScript`)
  (`MeshComponent.SetVectorParameterValueOnMaterials` (`self.StaticMesh`) "Color" (`KismetMathLibrary.Conv_LinearColorToVector` (struct :`G` 1.0 :`B` 0.134287 :`A` 1.0)))
  (`MeshComponent.SetVectorParameterValueOnMaterials` (`self.StaticMesh+`) "Color" (`KismetMathLibrary.Conv_LinearColorToVector` (struct :`G` 1.0 :`B` 0.134287 :`A` 1.0)))
  (`MeshComponent.SetVectorParameterValueOnMaterials` (`self.StaticMesh1`) "Color" (`KismetMathLibrary.Conv_LinearColorToVector` (struct :`R` 0.38125 :`G` 1.0 :`A` 1.0)))
  (`MeshComponent.SetVectorParameterValueOnMaterials` (`self.StaticMesh+1`) "Color" (`KismetMathLibrary.Conv_LinearColorToVector` (struct :`R` 0.38125 :`G` 1.0 :`A` 1.0)))
  (`MeshComponent.SetVectorParameterValueOnMaterials` (`self.StaticMesh2`) "Color" (`KismetMathLibrary.Conv_LinearColorToVector` (struct :`G` 1.0 :`B` 0.603235 :`A` 1.0)))
  (`MeshComponent.SetVectorParameterValueOnMaterials` (`self.StaticMesh+2`) "Color" (`KismetMathLibrary.Conv_LinearColorToVector` (struct :`G` 1.0 :`B` 0.603235 :`A` 1.0))))