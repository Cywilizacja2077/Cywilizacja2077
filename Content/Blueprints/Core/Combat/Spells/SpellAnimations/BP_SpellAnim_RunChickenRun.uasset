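; Spell animation actor for Run Chicken Run that shows the spell's icon over the target tile.
; On play, it moves to the target tile and sets the icon texture on its W_Image widget component.
; A timeline animates the widget's height, draw size and opacity, signals the tile hit once playback passes an early threshold, and completes the spell animation when finished.
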(event `self.Event_PlaySpellAnimation`
  (bind _widget (`self.Widget`))
  (bind _transform_location (`KismetMathLibrary.BreakTransform` (`self.GetTileTrasform` (`self.TargetIndex`))))
  (`self.K2_SetActorLocation` _transform_location)
  (bind _output_get (set `self.W Image` (cast `/Game/Blueprints/Core/Combat/Spells/SpellAnimations/Components/W_Image` (`WidgetComponent.GetUserWidgetObject` (`self.Widget`)) :!pure true)))
  (`Image.SetBrushFromTexture` (`/Game/Blueprints/Core/Combat/Spells/SpellAnimations/Components/W_Image.Image_Component` _output_get) "/Game/Blueprints/Core/Combat/Spells/SpellAnimations/Assets/Icon_RunChickenRun_NoBackground.Icon_RunChickenRun_NoBackground" false)
  (bind (_direction _locationz _drawsize _opacity) (`Timeline|Timeline` :!via `PlayFromStart`)
    (:`Update`
      (`SceneComponent.K2_SetRelativeLocation` _widget (`KismetMathLibrary.MakeVector` 0.0 0.0 _locationz) false false)
      (`WidgetComponent.SetDrawSize` _widget (`KismetMathLibrary.MakeVector2D` _drawsize _drawsize))
      (`Widget.SetRenderOpacity` (`self.W Image`) _opacity)
      (if (> (`TimelineComponent.GetPlaybackPosition` (`self.Timeline`)) 0.2)
        (`/Engine/EditorBlueprintResources/StandardMacros.DoOnce` false
          (:`Completed`
            (`self.OnAnimationHitTile` self (`self.TargetIndex`))))))
    (:`Finished`
      (`self.Event_CompleteSpellAnimation`))))

(fn `UserConstructionScript`
  (`parent.UserConstructionScript`))