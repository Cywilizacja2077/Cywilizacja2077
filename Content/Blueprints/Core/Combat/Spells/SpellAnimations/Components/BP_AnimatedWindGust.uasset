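; Animated wind gust spell visual actor that plays a one-shot movement and fade, then destroys itself shortly afterwards.
; Construction gives the mesh two translucent dynamic materials, with green colors multiplied by a random factor currently fixed at zero.
; A rate-adjustable timeline interpolates the actor from origin to target transform and drives material opacity.
; Partway through playback, a DoOnce signals shape animation completion before the timeline finishes.
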(event `self.ReceiveBeginPlay`
  (`TimelineComponent.SetPlayRate` (`self.Timeline_PlayAnimation`) (`self.PlayRate`))
  (bind (_direction _transformalpha _opacity) (`Timeline|Timeline_PlayAnimation` :!via `PlayFromStart`)
    (:`Update`
      (`self.K2_SetActorTransform` (`KismetMathLibrary.TLerp` (`self.OriginTransform`) (`self.TargetTransform`) _transformalpha))
      (`MeshComponent.SetScalarParameterValueOnMaterials` (`self.AnimatedWindGust`) "Opacity" _opacity)
      (if (> (`TimelineComponent.GetPlaybackPosition` (`self.Timeline_PlayAnimation`)) 0.35)
        (`/Engine/EditorBlueprintResources/StandardMacros.DoOnce` false
          (:`Completed`
            (`self.OnShapeAnimationCompleted` self)))))
    (:`Finished`
      (`KismetSystemLibrary.Delay` 0.5)
      (`self.K2_DestroyActor`))))

(fn `UserConstructionScript`
  (bind _returnvalue (`PrimitiveComponent.CreateDynamicMaterialInstance` (`self.AnimatedWindGust`) 0 "/Engine/Engine_MI_Shaders/M_Shader_SimpleTranslucent.M_Shader_SimpleTranslucent" "None"))
  (`MaterialInstanceDynamic.SetVectorParameterValue` _returnvalue "Color" (* (struct :`R` 0.062236 :`G` 0.411458 :`A` 1.0) (`KismetMathLibrary.RandomFloatInRange` 0.0)))
  (bind _returnvalue_2 (`PrimitiveComponent.CreateDynamicMaterialInstance` (`self.AnimatedWindGust`) 1 "/Engine/Engine_MI_Shaders/M_Shader_SimpleTranslucent.M_Shader_SimpleTranslucent" "None"))
  (`MaterialInstanceDynamic.SetVectorParameterValue` _returnvalue_2 "Color" (* (struct :`R` 0.151258 :`G` 1.0 :`A` 1.0) (`KismetMathLibrary.RandomFloatInRange` 0.0))))